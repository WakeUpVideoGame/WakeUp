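; Player character with collectible power-ups, checkpoint respawning and a pause menu.
; Overlaps call CollectPowers; PowerUp eases PowerLevel up on a timeline, then calls ActivatePower, while Tick feeds the level into a dynamic mesh material.
; On destruction (F forces it), it spawns and possesses a new MyCharacter at LastCheckpoint, falling back to the first PlayerStart found when none is set.
; The Random spawn option does not actually randomize.
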(event `InputAction|PauseMenu`
  (:`Pressed`
    (`GameplayStatics.SetGamePaused` null true)
    (bind _returnvalue (`|CreateWidget` "/Game/Blueprints/BP_PauseMenu.BP_PauseMenu_C"))
    (`UserWidget.AddToViewport` _returnvalue)
    (set `PlayerController.bShowMouseCursor` true (`GameplayStatics.GetPlayerController` null))))

(event `self.ReceiveActorBeginOverlap`
  (params (OtherActor :type "Actor Object Reference"))
  (`self.CollectPowers`))

(event `self.PowerUp`
  (params (PowerPickupLevel :type "Float (single-precision)"))
  (bind _powerlevel (`self.PowerLevel`))
  (set `self.PrechargePowerLevel` _powerlevel)
  (set `self.ResultingPowerLevel` (+ PowerPickupLevel _powerlevel))
  (bind (_direction _powerupcurve) (`Timeline|PowerUpTimeline` :!via `PlayFromStart`)
    (:`Update`
      (set `self.PowerLevel` (`KismetMathLibrary.Lerp` (`self.PrechargePowerLevel`) (`self.ResultingPowerLevel`) _powerupcurve)))
    (:`Finished`
      (`self.ActivatePower`))))

(event `self.ReceiveTick`
  (params (DeltaSeconds :type "Float (single-precision)"))
  (`parent.ReceiveTick` DeltaSeconds)
  (`MaterialInstanceDynamic.SetScalarParameterValue` (`self.DynamicPowerMaterial`) "PowerMultiplier" (`self.PowerLevel`)))

(event `self.ReceiveDestroyed`
  ;[0.06192 1 0] Respawn Player
  (`self.Spawn Player` "MyCharacter_C" (`self.Last Checkpoint`)))

(event `Key|F`
  ;[1 0 0] Tue le perso
  (:`Pressed`
    (`self.K2_DestroyActor`)))

(fn `Get Checkpoint`
  (returns (Location :type "Object.Transform Structure") (`Have Location` :type Boolean))
  (bind _last_checkpoint (`self.Last Checkpoint`))
  (return _last_checkpoint (!= (.location _last_checkpoint) (0.0 0.0 0.0))))

(fn `Set Checkpoint`
  (params (Update :type Boolean))
  (returns (Updated :type Boolean))
  (bind _returnvalue (`self.GetTransform`))
  (if Update
    (set `self.Last Checkpoint` _returnvalue)
    (else
      (set `self.Last Checkpoint` (struct))))
  (return (!= (.location _returnvalue) (0.0 0.0 0.0))))

(fn `Spawn Player`
  (params (Class :type "Actor Class Reference") (Transform :type "Object.Transform Structure") (Random :type Boolean))
  (bind _playerpawn (`self.playerPawn`))
  (if (!= (.location Transform) (0.0 0.0 0.0))
    (bind _returnvalue (`|SpawnActorFromClass` Class Transform))
    (bind _aspawn (cast `Pawn` _returnvalue))
    (set `self.playerPawn` _aspawn)
    (else
      (bind _outactors (`GameplayStatics.GetAllActorsOfClass` null "/Script/Engine.PlayerStart"))
      (if Random
        (bind _asplayerstart (cast `PlayerStart` (`KismetArrayLibrary.Array_Get` _outactors)))
        (set `self.lastSpawn` _asplayerstart)
        (else
          (for _array_element _outactors
            (bind _asplayerstart_2 (cast `PlayerStart` _array_element))
            (set `self.lastSpawn` _asplayerstart_2)
            (break))))
      (bind _returnvalue_2 (`|SpawnActorFromClass` Class (`self.GetTransform` (`self.lastSpawn`))))
      (bind _aspawn_2 (cast `Pawn` _returnvalue_2))
      (set `self.playerPawn` _aspawn_2)))
  (`self.SpawnDefaultController` _playerpawn)
  (`Controller.Possess` (`GameplayStatics.GetPlayerController` null) _playerpawn))

(fn `UserConstructionScript`
  (`|ExecutionSequence`
    (:`then_0`
      (bind _returnvalue (`PrimitiveComponent.CreateDynamicMaterialInstance` (`self.Mesh`) 0 null))
      (set `self.DynamicPowerMaterial` _returnvalue)
      (set `self.InitialPowerLevel` (`self.PowerLevel`)))
    (:`then_1`
      (set `self.playerpawn` (`GameplayStatics.GetPlayerPawn` null)))))