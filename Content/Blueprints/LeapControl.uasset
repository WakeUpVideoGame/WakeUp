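; Leap Motion control Blueprint that turns hand swipes into movement speed for WakeUpCharacter and visualizes the tracked arm.
; BeginPlay enables swipe gestures, and each detected swipe copies its speed to the character's MovementSpeed.
; Hand movement draws debug spheres at elbow and wrist, offset and rotated by control rotation, plus the actor rotation's X vector.
; The generic GestureDetected handler only casts to a swipe, with no further action.
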(event `self.LeapHandMoved`
  (params (hand :type "LeapHand Object Reference"))
  (bind _arm (`LeapHand.Arm` hand))
  (`self.Draw Debug Sphere At Actor` (`LeapArm.ElbowPosition` _arm) 2.0)
  (`self.Draw Debug Sphere At Actor` (`LeapArm.WristPosition` _arm) 4.0))

(event `self.ReceiveBeginPlay`
  ;[1 1 1] Get Gestures
  (`LeapController.EnableGesture` (`self.LeapController`) "GESTURE_TYPE_SWIPE" true))

(event `self.GestureDetected`
  (params (gesture :type "LeapGesture Object Reference"))
  ;[1 1 1] Cast To swipe
  (switch `LeapGesture.LeapGestureType` (`LeapGesture.Type` gesture)
    (:`GESTURE_TYPE_SWIPE`
      (cast `LeapSwipeGesture` gesture))))

(event `self.SwipeGestureDetected`
  (params (gesture :type "LeapSwipeGesture Object Reference"))
  ;[1 1 1] MovementSpeed
  (set `WakeUpCharacter.MovementSpeed` (`LeapSwipeGesture.Speed` gesture) (`self.WakeUpCharacter`)))

(fn `Draw Debug Sphere At Actor`
  (params (Location :type "Object.Vector Structure") (Radius :type "Float (double-precision)"))
  (`KismetSystemLibrary.DrawDebugSphere` (+ (`KismetMathLibrary.GreaterGreater_VectorRotator` (+ Location (75.0 0.0 -20.0)) (`self.GetControlRotation`)) (`KismetMathLibrary.Conv_RotatorToVector` (`self.K2_GetActorRotation`))) Radius))

(fn `UserConstructionScript`)