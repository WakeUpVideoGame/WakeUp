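; BP_Stick is an interactive stick switch that flips between activated and deactivated when something overlaps its Trigger.
; Each overlap plays or reverses the ActionStick timeline based on IsActivated, and the timeline drives the roll of StickMesh.
; When the timeline finishes, it toggles IsActivated and calls the StickActivated dispatcher, so listeners are notified of changes in both directions.
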(event `self.Trigger.OnComponentBeginOverlap`
  (params (OtherActor :type "Actor Object Reference") (OtherComp :type "PrimitiveComponent Object Reference") (OtherBodyIndex :type Integer) (bFromSweep :type Boolean) (SweepResult :type "EngineTypes.HitResult Structure (by ref)"))
  (if (`self.isActivated`)
    (bind (_direction _rotation) (`Timeline|ActionStick` :!via `Reverse` :!label _label)
      (:`Update`
        (`SceneComponent.SetRelativeRotation` (`self.StickMesh`) (`KismetMathLibrary.MakeRot` 0.0 0.0 _rotation) false))
      (:`Finished`
        (if (`self.isActivated`)
          (set `self.isActivated` false)
          (else
            (set `self.isActivated` true)))
        (`self.Stick activated`)))
    (else
      (goto _label))))

(fn `UserConstructionScript`)